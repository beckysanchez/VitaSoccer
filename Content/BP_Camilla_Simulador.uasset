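; Stretcher actor for a rescue simulator: the player loads a patient, then carries it to a goal zone.
; Two trigger boxes toggle its input for BP_Jugador_Final.
; E/gamepad-left snaps the first SkeletalMeshActor found onto it, lying down, enabling carrying after a delay.
; F/gamepad-bottom attaches it to a player facing opposite its forward (dot-product check), showing their bar UI, and releases it only inside BP_ZonaMeta, ending the mission.
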(event `Key|Gamepad_FaceButton_Bottom`
  (params (Key :type "Key Structure"))
  (bind _returnvalue (`GameplayStatics.GetPlayerPawn` 0))
  (bind _returnvalue_2 (`GameplayStatics.GetPlayerPawn` 0))
  (:`Pressed`
    (if (`self.MisionTerminada`) :!label _label
      (`KismetSystemLibrary.PrintString` "¡El jugador ya está a salvo!")
      (elif (`self.PacienteListo`)
        (if (`self.EstaAgarrada`)
          (bind _outactors (`GameplayStatics.GetAllActorsOfClass` "/Game/BP_ZonaMeta.BP_ZonaMeta_C"))
          (if (`self.IsOverlappingActor` (`|GetArrayItem` _outactors) _returnvalue_2)
            (`self.K2_DetachFromActor` "KeepWorld" "KeepWorld" "KeepWorld")
            (`self.K2_AddActorLocalOffset` (-20.0 20.0 -35.0))
            (bind _asbp_jugador_final (cast `/Game/BP_Jugador_Final` _returnvalue_2))
            (`Widget.RemoveFromParent` (`/Game/BP_Jugador_Final.BarraUI_Ref` _asbp_jugador_final))
            (set `/Game/BP_Jugador_Final.agarrandoCamilla` false _asbp_jugador_final)
            (set `self.MisionTerminada` true)
            (set `self.EstaAgarrada` false)
            (else
              (`KismetSystemLibrary.PrintString` "Falló")))
          (elif (< (`KismetMathLibrary.Dot_VectorVector` (`self.GetActorForwardVector` (`GameplayStatics.GetPlayerPawn` 0)) (`self.GetActorForwardVector`)) -0.7)
            (`self.K2_AttachToActor` self _returnvalue "None" "KeepWorld" "KeepWorld" "KeepWorld" true)
            (`self.K2_AddActorLocalOffset` (20.0 -20.0 35.0))
            (set `self.EstaAgarrada` true)
            (bind _asbp_jugador_final_2 (cast `/Game/BP_Jugador_Final` _returnvalue))
            (bind _barraui_ref (`/Game/BP_Jugador_Final.BarraUI_Ref` _asbp_jugador_final_2))
            (`/Engine/EditorBlueprintResources/StandardMacros.IsValid` _barraui_ref
              (:`Is Valid`
                (`UserWidget.AddToViewport` _barraui_ref 0)
                (set `/Game/BP_Jugador_Final.agarrandoCamilla` true _asbp_jugador_final_2)
                (set `/Game/BP_Jugador_Final.Referencia Camilla` self _asbp_jugador_final_2)))
            (else
              (`KismetSystemLibrary.PrintString` "Ponte de frente para cargar la camilla"))))))))

(event `Key|F`
  (params (Key :type "Key Structure"))
  (:`Pressed`
    (goto _label)))

(event `Key|Gamepad_FaceButton_Left`
  (params (Key :type "Key Structure"))
  (:`Pressed`
    (`/Engine/EditorBlueprintResources/StandardMacros.DoOnce` false :!label _label_2
      (:`Completed`
        (bind _returnvalue (`GameplayStatics.GetActorOfClass` "/Script/Engine.SkeletalMeshActor"))
        (`SkeletalMeshComponent.PlayAnimation` (`SkeletalMeshActor.SkeletalMeshComponent` _returnvalue) "/Game/Characters/Futbolista/Animaciones/Lying_Down.Lying_Down" false)
        (`self.K2_AttachToComponent` _returnvalue (`self.Punto_Jugador`) "None" "SnapToTarget" "SnapToTarget" "KeepWorld" true)
        (`KismetSystemLibrary.Delay` 6.0)
        (set `self.PacienteListo` true)))))

(event `Key|E`
  (params (Key :type "Key Structure"))
  (:`Pressed`
    (goto _label_2)))

(event `self.Box.OnComponentBeginOverlap`
  (params (OverlappedComponent :type "PrimitiveComponent Object Reference") (OtherActor :type "Actor Object Reference") (OtherComp :type "PrimitiveComponent Object Reference") (OtherBodyIndex :type Integer) (bFromSweep :type Boolean) (SweepResult :type "HitResult Structure (by ref)"))
  (cast `/Game/BP_Jugador_Final` OtherActor)
  (`self.EnableInput` (`GameplayStatics.GetPlayerController` 0) :!label _label_3))

(event `self.Box1.OnComponentBeginOverlap`
  (params (OverlappedComponent :type "PrimitiveComponent Object Reference") (OtherActor :type "Actor Object Reference") (OtherComp :type "PrimitiveComponent Object Reference") (OtherBodyIndex :type Integer) (bFromSweep :type Boolean) (SweepResult :type "HitResult Structure (by ref)"))
  (cast `/Game/BP_Jugador_Final` OtherActor)
  (goto _label_3))

(event `self.Box.OnComponentEndOverlap`
  (params (OverlappedComponent :type "PrimitiveComponent Object Reference") (OtherActor :type "Actor Object Reference") (OtherComp :type "PrimitiveComponent Object Reference") (OtherBodyIndex :type Integer))
  (cast `/Game/BP_Jugador_Final` OtherActor)
  (`self.DisableInput` (`GameplayStatics.GetPlayerController` 0) :!label _label_4))

(event `self.Box1.OnComponentEndOverlap`
  (params (OverlappedComponent :type "PrimitiveComponent Object Reference") (OtherActor :type "Actor Object Reference") (OtherComp :type "PrimitiveComponent Object Reference") (OtherBodyIndex :type Integer))
  (cast `/Game/BP_Jugador_Final` OtherActor)
  (goto _label_4))

(fn `UserConstructionScript`)