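; Player character for a stretcher-balancing simulator, driven by an Arduino controller over a serial port and by standard inputs.
; Tick parses serial messages into button actions on BP_Camilla_Simulador, tilt and joystick movement.
; While carrying, random target angles after rests are countered by tilt, updating stability and the balance widget; sustained error ends the mission and triggers vibration.
; Gazing at a PuntoInicio-tagged actor starts joystick play with a long vibration.
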(event Custom|Procesar_Mensaje_Arduino
  (params (Mensaje :type String))
  (bind _returnvalue (Utilities|String|Trim Mensaje))
  (bind _returnvalue_2 (Utilities|String|RightChop _returnvalue 2))
  (bind _returnvalue_3 (Utilities|String|ParseIntoArray _returnvalue_2 ","))
  (if (Utilities|Enum|Equal(Enum) _returnvalue "JB")
    (Development|PrintString "Jalo Boton")
    (bind _outactors (Actor|GetAllActorsOfClass "/Game/BP_Camilla_Simulador.BP_Camilla_Simulador_C"))
    (bind _asbp_camilla_simulador (Utilities|Casting|CastToBP_Camilla_Simulador (Utilities|Array|Get(acopy) _outactors)))
    (Default|ArduinoBotonCamilla _asbp_camilla_simulador)
    (elif (Utilities|Enum|Equal(Enum) _returnvalue "B")
      (Development|PrintString "Boton Animar")
      (bind _outactors_2 (Actor|GetAllActorsOfClass "/Game/BP_Camilla_Simulador.BP_Camilla_Simulador_C"))
      (bind _asbp_camilla_simulador_2 (Utilities|Casting|CastToBP_Camilla_Simulador (Utilities|Array|Get(acopy) _outactors_2)))
      (Default|ArduinoBotonAnimar _asbp_camilla_simulador_2)
      (elif (Utilities|String|StartsWith _returnvalue "G:")
        (bind _output_get (Variables|Default|SetValorGiroArduino (Math|Conversions|ToFloat(Integer) _returnvalue_2)))
        (Development|PrintString (Utilities|String|ToString(Float) _output_get))
        (elif (Utilities|String|StartsWith _returnvalue "J:")
          (bind _output_get_2 (Variables|Default|SetJoyStick%20X (Math|Conversions|ToFloat(Integer) (Utilities|Array|Get(acopy) _returnvalue_3))))
          (bind _output_get_3 (Variables|Default|SetJoyStick%20Y (Math|Conversions|ToFloat(Integer) (Utilities|Array|Get(acopy) _returnvalue_3 1))))
          (Variables|Default|SetJoyStick%20Y (/ _output_get_3 1e+02))
          (Variables|Default|SetJoyStick%20X (/ _output_get_2 1e+02)))))))

(event Custom|Leer_Serial
  ;[0.15 0.15 0.15 0.5] Coneccion
  (bind (_bsuccess _returnvalue) (Class|Serial|Readln (Variables|Default|GetPuertoSerial)))
  (if _bsuccess
    (bind _output_get (Variables|Default|SetMensajeSerial _returnvalue))
    (CallFunction|ProcesarMensajeArduino _output_get)
    (CallFunction|LeerSerial)))

(event Custom|Vibrar
  (Class|Serial|Println (Variables|Default|GetPuertoSerial) "VIBRAR"))

(event Custom|Vibrar%20Largo
  (Class|Serial|Println (Variables|Default|GetPuertoSerial) "VIBRAR_LARGO"))

(event EventBeginPlay
  (bind (_bopened _returnvalue) (Class|Serial|OpenComPort 6 115200))
  (Variables|Default|SetPuertoSerial _returnvalue)
  (Variables|Default|SetPuertoSerialAbierto _bopened)
  (Variables|Default|SetEn%20Descanso true)
  (Variables|Default|SetTimer%20Descanso 0.0)
  (Development|PrintString "SERIAL ABIERTO")
  (Input|AddMappingContext (PlayerController|LocalPlayerSubsystems|GetEnhancedInputLocalPlayerSubsystem (Game|GetPlayerController 0)) "/Game/VRTemplate/Input/IMC_Default.IMC_Default" 10 "(bIgnoreAllPressedKeysUntilRelease=True,bForceImmediately=False,bNotifyUserSettings=False)")
  (bind _returnvalue_2 (UserInterface|CreateWidget "/Game/WBP_Estabilizador.WBP_Estabilizador_C"))
  (Variables|Default|SetBarraUI_Ref _returnvalue_2)
  (Development|PrintString "barra")
  (Class|HeadMountedDisplayFunctionLibrary|SetTrackingOrigin "LocalFloor"))

(event Collision|EventActorBeginOverlap
  (params (OtherActor :type Actor%20Object%20Reference)))

(event EventEndPlay
  (params (EndPlayReason :type EEndPlayReason%20Enum :default "Destroyed"))
  (Class|Serial|Close (stale EventBeginPlay _returnvalue))
  (Variables|Default|SetPuertoSerialAbierto false))

(event EventTick
  (params (DeltaSeconds :type Float%20%28single-precision%29))
  (bind _returnvalue (Game|GetPlayerCameraManager 0))
  (bind _returnvalue_2 (Transformation|GetActorLocation _returnvalue))
  (Utilities|FlowControl|Sequence
    (:then_0
      ;[0.15 0.15 0.15 0.5] Coneccion
      (if (Variables|Default|GetPuertoSerialAbierto)
        (CallFunction|LeerSerial)))
    (:then_1
      ;[0.15 0.15 0.15 0.5] Movimiento
      (Utilities|FlowControl|Gate true
        (:Exit
          (Pawn|Input|AddMovementInput (Math|Vector|GetForwardVector (Math|Rotator|MakeRotator 0.0 0.0 (.Yaw (Math|Rotator|BreakRotator (Pawn|GetControlRotation :!class /Script/Engine.Pawn))))) 1.0 false))))
    (:then_2
      ;[0.03434 0.03434 0.03434] Balanceo
      (bind _output_get (Variables|Default|SetAngulo%20Actual (Math|Interpolation|FInterpTo (Variables|Default|GetAngulo%20Actual) (Variables|Default|GetAnguloObjetivo) (Utilities|Time|GetWorldDeltaSeconds) (Variables|Default|GetVelocidad%20Correccion))))
      (if (Variables|Default|GetagarrandoCamilla)
        (Transformation|SetRelativeRotation (Variables|/Game/BP_Camilla_Simulador.BP_Camilla_Simulador_C|GetPivote_Perfecto (Variables|Default|GetReferencia%20Camilla)) (Math|Rotator|MakeRotator (+ _output_get (* (Variables|Default|GetValorGiroArduino) -1.0)) 0.0 0.0) false false)))
    (:then_3
      ;[0.15 0.15 0.15 0.5] JoyStick Movimiento
      (if (Variables|Default|GetJuego%20Iniciado)
        (Pawn|Input|AddMovementInput (Transformation|GetActorForwardVector) (Variables|Default|GetJoyStick%20X) false)
        (Pawn|Input|AddMovementInput (Transformation|GetActorRightVector) (Variables|Default|GetJoyStick%20Y) false)))
    (:then_4
      ;[0.15 0.15 0.15 0.5] LOGICA BALANCEO NO TOCAR
      (if (Variables|Default|GetagarrandoCamilla)
        (if (Variables|Default|GetEn%20Descanso)
          (bind _output_get_2 (Variables|Default|SetTimer%20Descanso (+ (Variables|Default|GetTimer%20Descanso) (Utilities|Time|GetWorldDeltaSeconds))))
          (if (>= _output_get_2 3.0)
            (Development|PrintString "Descanso Terminado")
            (Variables|Default|SetEn%20Descanso false)
            (Variables|Default|SetTimer%20Descanso 0.0)
            (Variables|Default|SetAnguloObjetivo (Math|Random|RandomFloatinRange -3e+01 3e+01))
            (bind _output_get_3 (Variables|Default|SetError%20Balanceo (+ (Variables|Default|GetAnguloObjetivo) (* (Variables|Default|GetValorGiroArduino) -1.0)) :!label _label))
            (Variables|/Game/WBP_Estabilizador.WBP_Estabilizador_C|SetPosicionActual (Variables|Default|GetBarraUI_Ref) (Math|Float|MapRangeClamped _output_get_3 -3e+01 3e+01 0.0 1.0))
            (if (< (Math|Float|Absolute(Float) (Variables|Default|GetError%20Balanceo)) (Variables|Default|GetUmbral%20Estabilidad))
              (Variables|Default|SetEstabilidad (Math|Float|Clamp(Float) (+ (* (Utilities|Time|GetWorldDeltaSeconds) 15.0) (Variables|Default|GetEstabilidad)) 0.0 1e+02))
              (else
                (Variables|Default|SetEstabilidad (Math|Float|Clamp(Float) (- (* (Utilities|Time|GetWorldDeltaSeconds) 25.0) (Variables|Default|GetEstabilidad)) 0.0 1e+02))))
            (Variables|/Game/WBP_Estabilizador.WBP_Estabilizador_C|SetPosicionActual (Variables|Default|GetBarraUI_Ref) (Math|Float|MapRangeClamped (Variables|Default|GetError%20Balanceo) -3e+01 3e+01 0.0 1.0)))
          (elif (< (Math|Float|Absolute(Float) (Variables|Default|GetError%20Balanceo)) (Variables|Default|GetUmbral%20Estabilidad))
            (Variables|Default|SetTimer%20Fallo 0.0)
            (if (< (Math|Float|Absolute(Float) (Variables|Default|GetError%20Balanceo)) 5.0)
              (Variables|Default|SetEn%20Descanso true)
              (Variables|Default|SetTimer%20Descanso 0.0)
              (Variables|Default|SetAnguloObjetivo 0.0)
              (goto _label)
              (else
                (Variables|Default|SetTimer%20Fallo (Variables|Default|GetTimer%20Fallo))
                (goto _label)))
            (else
              (bind _output_get_4 (Variables|Default|SetTimer%20Fallo (+ (Variables|Default|GetTimer%20Fallo) (Utilities|Time|GetWorldDeltaSeconds))))
              (if (>= _output_get_4 (Variables|Default|GetLimite%20Fallo))
                (if (Variables|Default|GetagarrandoCamilla)
                  (Variables|/Game/BP_Camilla_Simulador.BP_Camilla_Simulador_C|SetMisionTerminada (Variables|Default|GetReferencia%20Camilla) true)
                  (Development|PrintString "Fallaste")
                  (CallFunction|Vibrar)
                  (Development|PrintString (Utilities|String|ToString(Float) (Variables|Default|GetError%20Balanceo)))
                  (goto _label))))))))
    (:then_5
      ;[0.15 0.15 0.15 0.5] Mirar a un objeto para iniciar el juego, quitar si no usas lentes
      (if (not (Variables|Default|GetJuego%20Iniciado))
        (bind (_outhit _returnvalue_3) (Collision|LineTraceByChannel _returnvalue_2 (+ (* (Transformation|GetActorForwardVector _returnvalue) (Math|Conversions|ToVector(Float) 5e+03)) _returnvalue_2) "TraceTypeQuery1" false 0 "None"))
        (if _returnvalue_3
          (bind _asactor (Utilities|Casting|CastToActor (.HitActor (Collision|BreakHitResult _outhit)))
            (:then
              _)
            (:CastFailed
              (Variables|Default|SetGaze%20timer 0.0)))
          (else
            (Variables|Default|SetGaze%20timer 0.0)))
        (if (Actor|ActorHasTag _asactor "PuntoInicio")
          (bind _output_get_5 (Variables|Default|SetGaze%20timer (+ (Variables|Default|GetGaze%20timer) (Utilities|Time|GetWorldDeltaSeconds))))
          (else
            (Variables|Default|SetGaze%20timer 0.0)))
        (if (>= _output_get_5 (Variables|Default|GetTiempo%20Requerido))
          (Variables|Default|SetJuego%20Iniciado true)
          (Input|EnableInput (Game|GetPlayerController 0))
          (CallFunction|VibrarLargo))))))

(event Input|AxisEvents|InputAxisMoveForward
  (params (AxisValue :type Float%20%28single-precision%29))
  (Pawn|Input|AddMovementInput (Transformation|GetActorForwardVector) AxisValue false))

(event Input|AxisEvents|InputAxisMoveRight
  (params (AxisValue :type Float%20%28single-precision%29))
  (Pawn|Input|AddMovementInput (Transformation|GetActorRightVector) AxisValue false))

(event Input|AxisEvents|InputAxisTurn
  (params (AxisValue :type Float%20%28single-precision%29))
  (Pawn|Input|AddControllerYawInput AxisValue))

(event Input|AxisEvents|InputAxisLookUp
  (params (AxisValue :type Float%20%28single-precision%29))
  (Pawn|Input|AddControllerPitchInput AxisValue))

(event Input|MouseEvents|MouseX
  (params (AxisValue :type Float%20%28single-precision%29))
  (Pawn|Input|AddControllerYawInput AxisValue))

(event Input|MouseEvents|MouseY
  (params (AxisValue :type Float%20%28single-precision%29))
  (Pawn|Input|AddControllerPitchInput (* AxisValue -1.0)))

(event Input|GamepadEvents|DebugKeyGamepadRightTrigger
  (params (Key :type Key%20Structure :default "None") (ActionValue :type Input%20Action%20Value%20Structure))
  (:Pressed
    (if (< (Math|Float|Absolute(Float) (Variables|/Game/WBP_Estabilizador.WBP_Estabilizador_C|GetPosicionActual (Variables|Default|GetBarraUI_Ref))) 0.2)
      (Variables|Default|SetEstabilidad 1e+02)
      (Development|PrintString "jaló")
      (else
        (Variables|Default|SetEstabilidad (- (Variables|Default|GetEstabilidad) 2e+01))
        (Development|PrintString "fallaste")))))

(event Input|KeyboardEvents|Q
  (params (Key :type Key%20Structure :default "None"))
  (:Pressed
    (if (< (Math|Float|Absolute(Float) (Variables|/Game/WBP_Estabilizador.WBP_Estabilizador_C|GetPosicionActual (Variables|Default|GetBarraUI_Ref))) 0.2)
      (Variables|Default|SetEstabilidad 1e+02)
      (Development|PrintString "jaló")
      (else
        (Variables|Default|SetEstabilidad (- (Variables|Default|GetEstabilidad) 2e+01))
        (Development|PrintString "fallaste")))))

(event Input|KeyboardEvents|W
  (params (Key :type Key%20Structure :default "None"))
  ;[0.15 0.15 0.15 0.5] Movimiento
  (:Pressed
    (Utilities|FlowControl|Gate true) ; enters at Open
  )
  (:Released
    (Utilities|FlowControl|Gate true) ; enters at Close
  ))

(fn ConstructionScript)