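; BP_ZonaMeta is a finish-zone trigger that ends the game when BP_Camilla_Simulador enters its Box.
; The overlap removes the BP_Jugador_Final bar UI, reveals PantallaVR and triggers a long vibration on the player.
; It then switches input to UI only and pauses the game.
; A separate actor-overlap event prints a win message once through DoOnce, without filtering the overlapping actor.
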(event `self.ReceiveActorBeginOverlap`
  (params (OtherActor :type "Actor Object Reference"))
  (`/Engine/EditorBlueprintResources/StandardMacros.DoOnce` false
    (:`Completed`
      (`KismetSystemLibrary.PrintString` "¡HAS GANADO!"))))

(event `self.Box.OnComponentBeginOverlap`
  (params (OverlappedComponent :type "PrimitiveComponent Object Reference") (OtherActor :type "Actor Object Reference") (OtherComp :type "PrimitiveComponent Object Reference") (OtherBodyIndex :type Integer) (bFromSweep :type Boolean) (SweepResult :type "HitResult Structure (by ref)"))
  (`KismetSystemLibrary.PrintString` "Toque la meta")
  (cast `/Game/BP_Camilla_Simulador` OtherActor)
  (bind _asbp_jugador_final (cast `/Game/BP_Jugador_Final` (`GameplayStatics.GetPlayerPawn` 0)))
  (`Widget.RemoveFromParent` (`/Game/BP_Jugador_Final.BarraUI_Ref` _asbp_jugador_final))
  (`SceneComponent.SetVisibility` (`self.PantallaVR`) true false)
  (bind _asbp_jugador_final_2 (cast `/Game/BP_Jugador_Final` (`GameplayStatics.GetPlayerPawn` 0)))
  (`/Game/BP_Jugador_Final.Vibrar Largo` _asbp_jugador_final_2)
  (`WidgetBlueprintLibrary.SetInputMode_UIOnlyEx` (`GameplayStatics.GetPlayerController` 0) null)
  (`GameplayStatics.SetGamePaused` true))

(fn `UserConstructionScript`)